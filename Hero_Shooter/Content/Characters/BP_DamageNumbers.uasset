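; BP_DamageNumbers is a short-lived actor that displays the damage total of its owning BP_TestDummy.
; Construction sets the DMG text from the dummy's DMGTotal, trimmed by character count according to magnitude, and caches its DamageCause.
; Each tick it rotates to face DamageCause, refreshing the text while Updating is true.
; It destroys itself after a brief delay from BeginPlay.
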(event EventTick
  (params (DeltaSeconds :type Float%20%28single-precision%29))
  (bind _returnvalue (Transformation|GetActorLocation))
  (bind _damage_cause (Variables|Default|GetDamage_Cause))
  (bind _returnvalue_2 (Transformation|GetActorLocation _damage_cause))
  (bind _returnvalue_3 (Math|Rotator|FindLookatRotation _returnvalue _returnvalue_2))
  (if (Variables|Default|GetUpdating)
    (Transformation|SetActorRotation _returnvalue_3)
    (CallFunction|TextUpdate (Components|GetOwner))
    (else
      (Transformation|SetActorRotation _returnvalue_3))))

(event EventBeginPlay
  (Utilities|FlowControl|Delay 2.5)
  (Actor|DestroyActor))

(fn ConstructionScript
  (Utilities|FlowControl|Sequence
    (:then_0
      (bind _asbp_test_dummy (CallFunction|TextUpdate (Components|GetOwner))))
    (:then_1
      (Variables|Default|SetDamage_Cause (Variables|/Game/Characters/Test_Dummy/BP_TestDummy.BP_TestDummy_C|GetDamage_Cause _asbp_test_dummy)))))

(fn TextUpdate
  (params (Object :type Object%20Object%20Reference))
  (bind _asbp_test_dummy (Utilities|Casting|CastToBP_TestDummy Object))
  (Rendering|Components|TextRender|SetText (Variables|Default|GetDMG) (Utilities|Text|ToText(String) (Utilities|String|Left (Utilities|String|ToString(Float) (Variables|/Game/Characters/Test_Dummy/BP_TestDummy.BP_TestDummy_C|GetDMGTotal _asbp_test_dummy)) (Math|Integer|SelectInt 5 4 (>= (Variables|/Game/Characters/Test_Dummy/BP_TestDummy.BP_TestDummy_C|GetDMGTotal _asbp_test_dummy) 1e+02)))))
  (return _asbp_test_dummy))