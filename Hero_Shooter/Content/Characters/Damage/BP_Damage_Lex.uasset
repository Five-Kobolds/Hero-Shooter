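; BP_Damage_Lex is the Lex character's shooting Blueprint, with ammo and crosshair widgets, automatic fire, reload and an ability.
; Primary fire opens a Tick-driven gate throttled by a FireSpeed Delay, spending ammo on debug-drawn camera line traces whose hits go unused.
; R refills ammo after a short delay.
; Ability 1 temporarily boosts fire rate and ammo, then restores fixed values, leaving Ability1Active set.
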(event EventTick
  (params (DeltaSeconds :type Float%20%28single-precision%29))
  (bind _camera (Variables|Default|GetCamera))
  (bind _returnvalue (Transformation|GetWorldLocation _camera))
  (Utilities|FlowControl|Gate true
    (:Exit
      (Utilities|FlowControl|Delay (Variables|Default|GetFireSpeed))
      (if (>= (Variables|Default|GetAmmo) 1)
        (bind _result (Math|Integer|DecrementInt (Variables|Default|GetAmmo))
          (:%20%20
            (Variables|Default|SetAmmo _result)
            (bind _outhit (Collision|LineTraceByChannel _returnvalue (+ _returnvalue (* (Math|Vector|GetForwardVector (Transformation|GetWorldRotation _camera)) 2e+03)) "TraceTypeQuery1" false 0 "ForDuration" false))))))))

(event EventBeginPlay
  (bind _returnvalue (UserInterface|CreateWidget "/Game/Characters/Damage/UI_Ammo.UI_Ammo_C"))
  (UserInterface|Viewport|AddtoViewport _returnvalue 0)
  (bind _returnvalue_2 (UserInterface|CreateWidget "/Game/UI/WP_Crossair.WP_Crossair_C"))
  (UserInterface|Viewport|AddtoViewport _returnvalue_2 0))

(event Input|ActionEvents|InputActionPrimaryfire
  (params (Key :type Key%20Structure :default "None"))
  (bind _camera (Variables|Default|GetCamera))
  (bind _returnvalue (Transformation|GetWorldLocation _camera))
  (:Pressed
    (Utilities|FlowControl|Gate true) ; enters at Open
  )
  (:Released
    (Utilities|FlowControl|Gate true) ; enters at Close
  ))

(event Input|ActionEvents|InputActionAbility1
  (params (Key :type Key%20Structure :default "None"))
  (:Pressed
    (Variables|Default|SetFireSpeed 0.06)
    (Variables|Default|SetAbility%201%20Active? true)
    (Variables|Default|SetAmmo 100)
    (Utilities|FlowControl|Delay 5.0)
    (Variables|Default|SetFireSpeed 0.3)
    (Variables|Default|SetAmmo 30)))

(event Input|ActionEvents|InputActionAbility2
  (params (Key :type Key%20Structure :default "None")))

(event Input|KeyboardEvents|R
  (params (Key :type Key%20Structure :default "None"))
  (:Pressed
    (Utilities|FlowControl|Delay 0.5)
    (Variables|Default|SetAmmo 30)))

(fn ConstructionScript
  (|CallParentFunction))