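; BP_Damage_Shoot is a damage-role player Blueprint with automatic hitscan fire, adding ammo and crosshair widgets on begin play.
; Holding Primary fire opens a Tick-driven Gate, where a Delay sets the fire rate for camera-forward debug line traces that consume ammo.
; R reloads after a delay, and Ability 1 temporarily boosts fire rate and ammo, then cools down.
; Trace hits are unused, so shots apply no damage.
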(event EventTick
  (params (DeltaSeconds :type Float%20%28single-precision%29))
  (bind _camera (Variables|Default|GetCamera))
  (bind _returnvalue (Transformation|GetWorldLocation _camera))
  (Utilities|FlowControl|Gate true
    (:Exit
      (Utilities|FlowControl|Delay (Variables|Default|GetDuration))
      (if (>= (Variables|Default|GetAmmo) 1)
        (bind _outhit (Collision|LineTraceByChannel _returnvalue (+ _returnvalue (* (Math|Vector|GetForwardVector (Transformation|GetWorldRotation _camera)) 1e+03)) "TraceTypeQuery1" false 0 "ForDuration" false))
        (bind _result (Math|Integer|DecrementInt (Variables|Default|GetAmmo))
          (:%20%20
            (Variables|Default|SetAmmo _result)))))))

(event EventBeginPlay
  (bind _returnvalue (Game|ConstructObjectfromClass "/Game/UI/UI_Ammo.UI_Ammo_C"))
  (UserInterface|Viewport|AddtoViewport _returnvalue 0)
  (bind _returnvalue_2 (Game|ConstructObjectfromClass "/Game/UI/WP_Crossair.WP_Crossair_C"))
  (UserInterface|Viewport|AddtoViewport _returnvalue_2 0))

(event Input|ActionEvents|InputActionPrimaryfire
  (params (Key :type Key%20Structure :default "None"))
  (bind _camera (Variables|Default|GetCamera))
  (bind _returnvalue (Transformation|GetWorldLocation _camera))
  (:Pressed
    (Utilities|FlowControl|Gate true) ; enters at Open
  )
  (:Released
    (Utilities|FlowControl|Gate true) ; enters at Close
  ))

(event Input|ActionEvents|InputActionAbility1
  (params (Key :type Key%20Structure :default "None"))
  (:Pressed
    (if (not (Variables|Default|GetIs%20Ability%201%20Active?))
      (Variables|Default|SetDuration 0.05)
      (Variables|Default|SetAmmo 100)
      (Variables|Default|SetIs%20Ability%201%20Active? true)
      (Utilities|FlowControl|Delay 5.0)
      (Variables|Default|SetDuration 0.3)
      (Variables|Default|SetAmmo 30)
      (Utilities|FlowControl|Delay 25.0)
      (Variables|Default|SetIs%20Ability%201%20Active? false))))

(event Input|KeyboardEvents|R
  (params (Key :type Key%20Structure :default "None"))
  (:Pressed
    (Utilities|FlowControl|Delay 0.5)
    (Variables|Default|SetAmmo 30)))

(fn ConstructionScript
  (|CallParentFunction))