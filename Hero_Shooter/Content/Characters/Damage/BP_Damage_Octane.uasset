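; Damage-type playable character Octane, with melee, slash, sidestep and speed-boost abilities fueled by a VoidGauge resource.
; Primary fire in SwordZone builds the gauge, dealing damage only when that gain reaches the cap; secondary fire spends it, damaging the actor in SlashZone.
; Q and LeftShift spend gauge on launch sidesteps, while Ability 2 buys a timed walk-speed boost.
; BeginPlay adds a crosshair widget, and Tick debug-prints the gauge.
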(event OnComponentEndOverlap(SwordZone)
  (params (OverlappedComponent :type Primitive%20Component%20Object%20Reference) (OtherActor :type Actor%20Object%20Reference) (OtherComp :type Primitive%20Component%20Object%20Reference) (OtherBodyIndex :type Integer))
  (Variables|Default|SetActorInFrontOfMe 0)
  (Variables|Default|SetInSwordZone? false))

(event OnComponentBeginOverlap(SwordZone)
  (params (OverlappedComponent :type Primitive%20Component%20Object%20Reference) (OtherActor :type Actor%20Object%20Reference) (OtherComp :type Primitive%20Component%20Object%20Reference) (OtherBodyIndex :type Integer) (bFromSweep :type Boolean) (SweepResult :type Hit%20Result%20Structure%20%28by%20ref%29))
  (Variables|Default|SetActorInFrontOfMe OtherActor)
  (Variables|Default|SetInSwordZone? true))

(event OnComponentBeginOverlap(SlashZone)
  (params (OverlappedComponent :type Primitive%20Component%20Object%20Reference) (OtherActor :type Actor%20Object%20Reference) (OtherComp :type Primitive%20Component%20Object%20Reference) (OtherBodyIndex :type Integer) (bFromSweep :type Boolean) (SweepResult :type Hit%20Result%20Structure%20%28by%20ref%29))
  (Variables|Default|SetActorInRange OtherActor)
  (Variables|Default|SetInSlashZone? true))

(event OnComponentEndOverlap(SlashZone)
  (params (OverlappedComponent :type Primitive%20Component%20Object%20Reference) (OtherActor :type Actor%20Object%20Reference) (OtherComp :type Primitive%20Component%20Object%20Reference) (OtherBodyIndex :type Integer))
  (Variables|Default|SetActorInRange 0)
  (Variables|Default|SetInSlashZone? false))

(event EventTick
  (params (DeltaSeconds :type Float%20%28single-precision%29))
  (Development|PrintString (Utilities|String|ToString(Integer) (Variables|Default|GetVoid%20Gauge))))

(event EventBeginPlay
  (bind _returnvalue (UserInterface|CreateWidget "/Game/UI/WP_Crossair.WP_Crossair_C"))
  (UserInterface|Viewport|AddtoViewport _returnvalue 0))

(event Input|ActionEvents|InputActionPrimaryfire
  (params (Key :type Key%20Structure :default "None"))
  (:Pressed
    (if (not (Variables|Default|GetIsAbility1Active?))
      (if (Variables|Default|GetInSwordZone?)
        (if (not (>= (Variables|Default|GetVoid%20Gauge) 100))
          (Variables|Default|SetVoid%20Gauge (+ (Variables|Default|GetVoid%20Gauge) 25))
          (if (>= (Variables|Default|GetVoid%20Gauge) 100)
            (Variables|Default|SetVoid%20Gauge 100)
            (Game|Damage|ApplyDamage (Variables|Default|GetActorInFrontOfMe) 2e+01 0 0 "/Script/Engine.DamageType")
            (Development|PrintString "Hit ")))))))

(event Input|ActionEvents|InputActionAbility2
  (params (Key :type Key%20Structure :default "None"))
  (bind _charactermovement (Variables|Character|GetCharacterMovement))
  (:Pressed
    (if (not (Variables|Default|GetIsAbility1Active?))
      (if (not (Variables|Default|GetIsAbility2Active?))
        (if (not (<= (stale _output_get) 29))
          (bind _output_get (Variables|Default|SetVoid%20Gauge (- (Variables|Default|GetVoid%20Gauge) 30)))
          (Variables|/Script/Engine.CharacterMovementComponent|SetMaxWalkSpeed _charactermovement 1e+03)
          (Variables|Default|SetIsAbility2Active? true)
          (Utilities|FlowControl|Delay 5.0)
          (Variables|/Script/Engine.CharacterMovementComponent|SetMaxWalkSpeed _charactermovement 6e+02)
          (Variables|Default|SetIsAbility2Active? false))))))

(event Input|ActionEvents|InputActionsecondaryfire
  (params (Key :type Key%20Structure :default "None"))
  (:Pressed
    (if (not (Variables|Default|GetIsAbility1Active?))
      (if (not (<= (stale _output_get) 19))
        (bind _output_get (Variables|Default|SetVoid%20Gauge (- (Variables|Default|GetVoid%20Gauge) 20)))
        (if (Variables|Default|GetInSlashZone?)
          (Game|Damage|ApplyDamage (Variables|Default|GetActorInRange) 2e+01 0 0 "/Script/Engine.DamageType")
          (Development|PrintString "Range Hit "))))))

(event Input|KeyboardEvents|Q
  (params (Key :type Key%20Structure :default "None"))
  (:Pressed
    (if (not (<= (stale _output_get) 49))
      (bind _output_get (Variables|Default|SetVoid%20Gauge (- (Variables|Default|GetVoid%20Gauge) 50)))
      (Character|LaunchCharacter (+ (* (Transformation|GetActorRightVector) (Variables|Default|GetSidestepRightForce)) (* (Transformation|GetActorUpVector) (Variables|Default|GetJump%20Force))) false false))))

(event Input|KeyboardEvents|LeftShift
  (params (Key :type Key%20Structure :default "None"))
  (:Pressed
    (if (not (<= (stale _output_get) 49))
      (bind _output_get (Variables|Default|SetVoid%20Gauge (- (Variables|Default|GetVoid%20Gauge) 50)))
      (Character|LaunchCharacter (+ (* (Transformation|GetActorRightVector) (Variables|Default|GetSidestepLeftForce)) (* (Transformation|GetActorUpVector) (Variables|Default|GetJump%20Force))) false false))))

(fn ConstructionScript
  (|CallParentFunction))