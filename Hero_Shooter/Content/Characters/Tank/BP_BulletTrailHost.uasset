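; Bullet trail host actor for the Tank character that animates a shot's travel from its spawn point to its end point, then removes itself.
; Trail_Init records the Sphere's world location, then a timeline curve lerps the root toward TargetLocation, or TraceEnd when the target is exactly zero.
; Movement ignores collision sweeps, and the actor destroys itself after a short delay once the timeline finishes.
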(event Custom|Trail_Init
  (params (Trace%20End :type Vector) (Target%20Location :type Vector))
  (bind _output_get (Variables|Default|SetInitial%20Location (Transformation|GetWorldLocation (Variables|Default|GetSphere))))
  (bind _travel_curve (Timeline|Travel%20Time PlayFromStart)
    (:Update
      (Transformation|SetWorldLocation (Variables|Default|GetDefaultSceneRoot) (Math|Vector|Lerp(Vector) _output_get (Math|Vector|SelectVector Trace%20End Target%20Location (Utilities|Operators|EqualEqual :A Target%20Location)) _travel_curve) false false))
    (:Finished
      (Utilities|FlowControl|Delay 0.5)
      (Actor|DestroyActor))))

(fn ConstructionScript)