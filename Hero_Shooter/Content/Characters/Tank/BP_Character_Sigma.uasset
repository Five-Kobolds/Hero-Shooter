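; Sigma tank character with a hitscan shotgun, deployable barrier and hook ability.
; Tick polls primary fire, line-tracing randomly spread pellets with distance falloff, tag-based headshots and impact effects; the older projectile loop is disconnected.
; Ability 1 toggles a barrier that shots ignore and stops moving on release; Ability 2 spawns a hook, gated by DoOnce and cooldown.
; Incoming damage scales by TankPassive, whose low-health check is never called here.
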(event Custom|FireReset
  (bind _projectile_source (Variables|Default|GetProjectile%20Source))
  (bind _returnvalue (Transformation|GetWorldTransform _projectile_source))
  ;[1 1 1] Outdated Projectile Script
  (Utilities|FlowControl|DoOnce false) ; enters at Reset
)

(event Custom|DestroyBarrier
  (bind _barrier_ref (Variables|Default|GetBarrier%20Ref))
  (Utilities|IsValid _barrier_ref
    (:Is%20Valid
      (Actor|DestroyActor _barrier_ref))))

(event Custom|Primary%20Fire
  (bind _spread (Variables|Default|GetSpread))
  (bind _spread_2 (Variables|Default|GetSpread))
  (bind _spread_3 (Variables|Default|GetSpread))
  (bind _projectile_source (Variables|Default|GetProjectile%20Source))
  (bind _returnvalue (Transformation|GetWorldLocation _projectile_source))
  (if (Variables|Default|GetPrimeFire)
    (|FireDelay)
    ;[1 1 1] For Each Pellet
    (for _index (range 0 5)
      (bind _outhit (Collision|LineTraceByChannel _returnvalue (+ _returnvalue (* (Math|Vector|GetForwardVector (Transformation|GetWorldRotation _projectile_source)) 1.5e+03) (Math|Vector|MakeVector (Math|Random|RandomFloatinRange (* _spread -1.0) _spread) (Math|Random|RandomFloatinRange (* _spread_3 -1.0) _spread_3) (Math|Random|RandomFloatinRange (* _spread_2 -1.0) _spread_2))) "TraceTypeQuery1" false (Variables|Default|GetShotgun%20Actors%20Ignore) "None"))
      (Utilities|IsValid (.hitactor _outhit)
        (:Is%20Valid
          (Utilities|FlowControl|Sequence
            (:then_0
              (CallFunction|DamageFalloff (.distance _outhit))
              (CallFunction|HeadshotDetection (.hitcomponent _outhit))
              (Game|Damage|ApplyDamage (.hitactor _outhit) (Math|Float|Clamp(Float) (* (Variables|Default|GetDamage) (Variables|Default|GetFalloff) (Variables|Default|GetHeadshot%20Multiplier)) 0.0 15.0) 0 self "/Engine/EngineDamageTypes/DmgTypeBP_Environmental.DmgTypeBP_Environmental_C"))
            (:then_1
              (CallFunction|BulletImpact))))))))

(event Custom|ResetHook
  (Utilities|FlowControl|DoOnce false) ; enters at Reset
)

(event Custom|HookActive
  (Utilities|FlowControl|DoOnce false) ; enters at Reset
)

(event Custom|Niagara%20Component%20Remove
  (params (Niagra%20System :type Niagara%20Component%20Object%20Reference))
  (Utilities|FlowControl|Delay 5.0)
  (Utilities|IsValid Niagra%20System
    (:Is%20Valid
      (Components|DestroyComponent Niagra%20System))))

(event Custom|Tank%20Passive%20Check
  (Variables|Default|SetTankPassive (Math|Float|SelectFloat 0.75 1.0 (<= (/ (Variables|Default|GetHealth) (Variables|Default|GetMaxHealth)) 0.25))))

(event Custom|Bullet_Impact
  (bind _returnvalue (Game|SpawnActorfromClass "/Game/Characters/Tank/BP_ShotgunImpact.BP_ShotgunImpact_C" (Math|Transform|MakeTransform (.location (stale Custom|Primary%20Fire _outhit)) "0, 0, 0" "0.250000,0.250000,0.250000") "Undefined" self 0))
  (Default|FacingDirection _returnvalue))

(event EventBeginPlay
  (bind _returnvalue (UserInterface|CreateWidget "/Game/Characters/Tank/WBP_Crosshair.WBP_Crosshair_C"))
  (bind _output_get (Variables|Default|SetCrosshair%20Ref _returnvalue))
  (UserInterface|Viewport|AddtoViewport _output_get 0)
  (bind _returnvalue_2 (UserInterface|CreateWidget "/Game/Defaults/WBP_TestUI.WBP_TestUI_C"))
  (bind _output_get_2 (Variables|Default|SetObjVal_Test _returnvalue_2))
  (UserInterface|Viewport|AddtoViewport _output_get_2 0))

(event Game|Damage|EventAnyDamage
  (params (Damage :type Float%20%28single-precision%29) (DamageType :type Damage%20Type%20Object%20Reference) (InstigatedBy :type Controller%20Object%20Reference) (DamageCauser :type Actor%20Object%20Reference))
  (bind _output_get (Variables|Default|SetHealth (Math|Float|Clamp(Float) (- (Variables|Default|GetHealth) (* Damage (Variables|Default|GetTankPassive))) 0.0 4e+02)))
  (if (<= _output_get 0.0)
    _))

(event EventTick
  (params (DeltaSeconds :type Float%20%28single-precision%29))
  (Utilities|FlowControl|Sequence
    (:then_0
      (Utilities|IsValid (Variables|Default|GetHook%20Ref)
        (:Is%20Not%20Valid
          (Utilities|FlowControl|DoOnce false
            (:Completed
              (Utilities|FlowControl|Delay (Variables|Default|GetAbilityCD2))
              (CallFunction|ResetHook))))))
    (:then_1
      (CallFunction|PrimaryFire))))

(event Input|ActionEvents|InputActionPrimaryfire
  (params (Key :type Key%20Structure :default "None"))
  (:Pressed
    (Variables|Default|SetPrimeFire true))
  (:Released
    (Variables|Default|SetPrimeFire false)))

(event Input|ActionEvents|InputActionAbility1
  (params (Key :type Key%20Structure :default "None"))
  (bind _barrier_source (Variables|Default|GetBarrier%20Source))
  (bind _returnvalue (Transformation|GetWorldTransform _barrier_source))
  (:Pressed
    (Utilities|FlowControl|FlipFlop
      (:A
        (bind _returnvalue_2 (Game|SpawnActorfromClass "/Game/Characters/Tank/BP_Deployable_Barrier.BP_Deployable_Barrier_C" (Math|Transform|MakeTransform (.location _returnvalue) (.rotation _returnvalue) "0.050000,2.000000,1.750000") "Undefined" self 0))
        (bind _output_get (Variables|Default|SetBarrier%20Ref _returnvalue_2))
        (Utilities|Array|Add (Variables|Default|GetShotgun%20Actors%20Ignore) _output_get))
      (:B
        (CallFunction|DestroyBarrier))))
  (:Released
    (bind _asbp_deployable_barrier (Utilities|Casting|CastToBP_Deployable_Barrier (Variables|Default|GetBarrier%20Ref)))
    (if (Utilities|IsValid _asbp_deployable_barrier)
      (Variables|/Game/Characters/Tank/BP_Deployable_Barrier.BP_Deployable_Barrier_C|SetStopMotion _asbp_deployable_barrier true))))

(event Input|ActionEvents|InputActionAbility2
  (params (Key :type Key%20Structure :default "None"))
  (:Pressed
    (Utilities|FlowControl|DoOnce false
      (:Completed
        (bind _returnvalue (Game|SpawnActorfromClass "/Game/Characters/Tank/BP_Hook.BP_Hook_C" (Transformation|GetWorldTransform (Variables|Default|GetProjectile%20Source)) "Undefined" self 0))
        (Variables|Default|SetHook%20Ref _returnvalue)
        (CallFunction|HookActive)))))

(event Input|KeyboardEvents|R
  (params (Key :type Key%20Structure :default "None"))
  (bind _tags (Variables|Default|GetTags))
  (:Pressed
    (Utilities|FlowControl|FlipFlop
      (:A
        (Utilities|Array|SetArrayElem _tags 0 "Team 1"))
      (:B
        (Utilities|Array|SetArrayElem _tags 0 "Team 2")))))

(fn ConstructionScript
  (|CallParentFunction)
  (Variables|Default|SetMaxHealth (Variables|Default|GetHealth)))

(fn HeadshotDetection
  (params (Hit%20Component :type Actor%20Component%20Object%20Reference))
  (bind _componenttags (Variables|/Script/Engine.ActorComponent|GetComponentTags Hit%20Component))
  (if (not (== (Utilities|Array|Length _componenttags) 0))
    (Variables|Default|SetHeadshot%20Multiplier (Math|Float|SelectFloat 2.0 1.0 (== (Utilities|Array|Get(acopy) _componenttags) "Head")))))

(fn DamageFalloff
  (params (HitDistance :type Float%20%28double-precision%29))
  (if (not (> HitDistance 1.5e+02))
    (Variables|Default|SetFalloff 1.0)
    (else
      (Variables|Default|SetFalloff (- 1.0 (/ HitDistance 1e+03))))))

(fn CableInit
  (params (Cable%20Reference :type Cable%20Component%20Object%20Reference))
  (Utilities|FlowControl|Sequence
    (:then_0
      (Variables|/Script/CableComponent.CableComponent|SetCableGravityScale Cable%20Reference 0.25))
    (:then_1
      (Variables|/Script/CableComponent.CableComponent|SetCableWidth Cable%20Reference 1.5))
    (:then_2
      (Variables|/Script/CableComponent.CableComponent|SetSolverIterations Cable%20Reference 10))
    (:then_3
      (Variables|/Script/CableComponent.CableComponent|SetEndLocation Cable%20Reference "0, 0, 0"))))