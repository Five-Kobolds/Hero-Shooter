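; Shotgun impact effect actor for the Tank character, showing a short-lived particle burst.
; Its Facing_Direction event turns the Arrow component toward the owner's camera, then destroys the actor after a brief delay.
; When the LowVisRange volume begins overlapping the owner, it hides the main ImpactParticle and shows ImpactLow instead, swapping the effect at close range.
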(event OnComponentBeginOverlap(LowVisRange)
  (params (OverlappedComponent :type Primitive%20Component%20Object%20Reference) (OtherActor :type Actor%20Object%20Reference) (OtherComp :type Primitive%20Component%20Object%20Reference) (OtherBodyIndex :type Integer) (bFromSweep :type Boolean) (SweepResult :type Hit%20Result%20Structure%20%28by%20ref%29))
  (if (== OtherActor (Components|GetOwner))
    (Rendering|SetVisibility (Variables|Default|GetImpact%20Particle) false false)
    (Rendering|SetVisibility (Variables|Default|GetImpact%20Low) true false)))

(event Custom|Facing_Direction
  (Transformation|SetWorldRotation (Variables|Default|GetArrow) (Math|Rotator|FindLookatRotation (Transformation|GetActorLocation) (Transformation|GetWorldLocation (Actor|GetComponentbyClass (Components|GetOwner) "/Script/Engine.CameraComponent"))) false false)
  (Utilities|FlowControl|Delay 0.5)
  (Actor|DestroyActor))

(fn ConstructionScript
  (if true
    _))