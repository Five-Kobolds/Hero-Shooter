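; BP_Shotgun_Pellet is a short-lived shotgun pellet that damages actors its sphere overlaps, with damage falling off over its flight time.
; Construction sets a half-second lifespan and copies the Damage value from its owning BP_Character_Sigma.
; On overlap, remaining lifespan stands in for distance: early hits deal full damage, later ones scale down toward zero.
; Damage is applied as environmental type, credited to the owner.
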(event OnComponentBeginOverlap(Sphere)
  (params (OverlappedComponent :type Primitive%20Component%20Object%20Reference) (OtherActor :type Actor%20Object%20Reference) (OtherComp :type Primitive%20Component%20Object%20Reference) (OtherBodyIndex :type Integer) (bFromSweep :type Boolean) (SweepResult :type Hit%20Result%20Structure%20%28by%20ref%29))
  (bind _returnvalue (Actor|GetLifeSpan))
  (bind _independantdamage (Variables|Default|GetIndependantDamage))
  (Game|Damage|ApplyDamage OtherActor (Math|Float|SelectFloat _independantdamage (* _independantdamage (* _returnvalue 2.0)) (> _returnvalue 0.375)) 0 (Components|GetOwner) "/Engine/EngineDamageTypes/DmgTypeBP_Environmental.DmgTypeBP_Environmental_C"))

(fn ConstructionScript
  (Actor|SetLifeSpan 0.5)
  (bind _asbp_character_sigma (Utilities|Casting|CastToBP_Character_Sigma (Components|GetOwner)))
  (Variables|Default|SetIndependantDamage (Variables|/Game/Characters/Character_Base.Character_Base_C|GetDamage _asbp_character_sigma)))