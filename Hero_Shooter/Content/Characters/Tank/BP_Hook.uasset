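; Tank character's hook projectile that flies out, then retracts to its launch point, dragging overlapped actors with it.
; It stores the cube's starting location and retracts after a short delay or on overlap, zeroing projectile velocity while the ComeBack timeline lerps the cube back.
; A second timeline lerps any overlapped actor to that point, with no filtering.
; When retraction finishes, it sets HookComplete and destroys itself.
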(event OnComponentBeginOverlap(Cube)
  (params (OverlappedComponent :type Primitive%20Component%20Object%20Reference) (OtherActor :type Actor%20Object%20Reference) (OtherComp :type Primitive%20Component%20Object%20Reference) (OtherBodyIndex :type Integer) (bFromSweep :type Boolean) (SweepResult :type Hit%20Result%20Structure%20%28by%20ref%29))
  (Utilities|FlowControl|Sequence
    (:then_0
      (bind _newtrack_0 (Timeline|ComeBack Play)
        (:Update
          (Variables|/Script/Engine.MovementComponent|SetVelocity (Variables|Default|GetProjectileMovement) "0, 0, 0")
          (Transformation|SetWorldLocation (Variables|Default|GetCube) (Math|Vector|Lerp(Vector) (Transformation|GetWorldLocation (Variables|Default|GetCube)) (stale EventBeginPlay _output_get) _newtrack_0) false false))
        (:Finished
          (Variables|Default|SetHookComplete? true)
          (Actor|DestroyActor))))
    (:then_1
      (bind _newtrack_0_2 (Timeline|Timeline_0 Play)
        (:Update
          (Transformation|SetWorldLocation (Variables|/Script/Engine.Actor|GetRootComponent OtherActor) (Math|Vector|Lerp(Vector) (Transformation|GetActorLocation OtherActor) (Variables|Default|GetLocation) _newtrack_0_2) false false))))))

(event EventBeginPlay
  (bind _cube (Variables|Default|GetCube))
  (bind _returnvalue (Transformation|GetWorldLocation _cube))
  (bind _output_get (Variables|Default|SetLocation _returnvalue))
  (Utilities|FlowControl|Delay 0.5)
  (bind _newtrack_0 (Timeline|ComeBack Play)
    (:Update
      (Variables|/Script/Engine.MovementComponent|SetVelocity (Variables|Default|GetProjectileMovement) "0, 0, 0")
      (Transformation|SetWorldLocation (Variables|Default|GetCube) (Math|Vector|Lerp(Vector) _returnvalue _output_get _newtrack_0) false false))
    (:Finished
      (Variables|Default|SetHookComplete? true)
      (Actor|DestroyActor))))

(fn ConstructionScript)