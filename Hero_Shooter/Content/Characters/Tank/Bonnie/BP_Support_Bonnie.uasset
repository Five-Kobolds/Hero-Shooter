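; Bonnie's playable character Blueprint, handling health, attacks and two abilities, with debug prints as feedback.
; Held inputs drive a box-overlap melee and an ammo-limited, reloadable hitscan shot, both sparing actors that share its first tag.
; Ability 1 temporarily boosts melee damage and speed.
; Holding Ability 2 blocks attacking and converts incoming damage into charge, split on release among non-allies in a sphere atop a base burst.
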(event Custom|primary
  (if (Variables|Default|Getfree)
    (if (Variables|Default|Getcan%20shoot)
      (for _array_element (Collision|GetOverlappingActors (Variables|Default|GetBox) 0 :!class /Script/Engine.PrimitiveComponent)
        (if (not (Actor|ActorHasTag _array_element (Utilities|Array|Get(acopy) (Variables|Default|GetTags))))
          (Game|Damage|ApplyDamage _array_element (Variables|Default|GetBase%20Damage) 0 0)
          (Development|PrintString (Utilities|GetDisplayName _array_element))
          (Variables|Default|Setcan%20shoot false)
          (Utilities|FlowControl|Delay 0.6)
          (Variables|Default|Setcan%20shoot true))))))

(event Custom|secondary
  (bind _ammo (Variables|Default|Getammo))
  (bind _camera (Variables|Default|GetCamera))
  (bind _returnvalue (Transformation|GetWorldLocation _camera))
  (if (Variables|Default|Getfree)
    (if (Variables|Default|Getcan%20shoot)
      (if (>= _ammo 1)
        (Variables|Default|Setcan%20shoot false)
        (Math|Integer|DecrementInt _ammo
          (:%20%20
            (Development|PrintString (Utilities|String|ToString(Integer) _ammo))
            (bind (_outhit _returnvalue_2) (Collision|LineTraceByChannel _returnvalue (+ _returnvalue (* (Math|Vector|GetForwardVector (Transformation|GetWorldRotation _camera)) 5e+03)) "TraceTypeQuery1" false 0 "ForDuration"))
            (if _returnvalue_2
              (Development|PrintString (Utilities|GetDisplayName (.hitactor _outhit)))
              (if (Actor|ActorHasTag (.hitactor _outhit) (Utilities|Array|Get(acopy) (Variables|Default|GetTags)))
                (Utilities|FlowControl|Delay 0.2 :!label _label)
                (Variables|Default|Setcan%20shoot true)
                (else
                  (Game|Damage|ApplyDamage (.hitactor _outhit) 15.0 0 0)
                  (Utilities|FlowControl|Delay 0.2)
                  (Variables|Default|Setcan%20shoot true)))
              (else
                (goto _label)))))
        (else
          (Development|PrintString "reload"))))))

(event EventTick
  (params (DeltaSeconds :type Float%20%28single-precision%29))
  (if (Variables|Default|Getm1)
    (CallFunction|Primary))
  (if (Variables|Default|Getm2)
    (CallFunction|Secondary)))

(event EventQuinnHighlight)

(event EventQuinnDehighlight)

(event Game|Damage|EventAnyDamage
  (params (Damage :type Float%20%28single-precision%29) (DamageType :type Damage%20Type%20Object%20Reference) (InstigatedBy :type Controller%20Object%20Reference) (DamageCauser :type Actor%20Object%20Reference))
  (if (Variables|Default|Getshield)
    (if (>= Damage 0.0)
      (bind _output_get (Variables|Default|Setcharge (+ (Variables|Default|Getcharge) Damage)))
      (Development|PrintString (Utilities|String|ToString(Float) _output_get)))
    (else
      (Variables|Default|SetHealth (- (Variables|Default|GetHealth) Damage))
      (Development|PrintString (Utilities|String|ToString(Float) Damage))
      (Development|PrintString (Utilities|String|ToString(Float) (Variables|Default|GetHealth))))))

(event EventQuinnCloud
  (Utilities|FlowControl|Delay 0.5)
  (Utilities|Array|RemoveItem (Variables|Default|GetTags) "EF"))

(event Input|ActionEvents|InputActionPrimaryfire
  (params (Key :type Key%20Structure :default "None"))
  (:Pressed
    (Variables|Default|Setm1 true))
  (:Released
    (Variables|Default|Setm1 false)))

(event Input|ActionEvents|InputActionReload
  (params (Key :type Key%20Structure :default "None"))
  (:Pressed
    (if (Variables|Default|Getfree)
      (Variables|Default|Setfree false)
      (if (< (Variables|Default|Getammo) 20)
        (Utilities|FlowControl|Delay 2.0)
        (Variables|Default|Setammo 20)
        (Development|PrintString (Utilities|String|ToString(Integer) (Variables|Default|Getammo)))
        (Variables|Default|Setfree true)
        (else
          (Variables|Default|Setfree true))))))

(event Input|ActionEvents|InputActionsecondaryfire
  (params (Key :type Key%20Structure :default "None"))
  (:Pressed
    (Variables|Default|Setm2 true))
  (:Released
    (Variables|Default|Setm2 false)))

(event Input|ActionEvents|InputActionAbility1
  (params (Key :type Key%20Structure :default "None"))
  (:Pressed
    (if (Variables|Default|Geta1cd)
      (Variables|Default|Seta1cd false)
      (Variables|Default|SetBase%20Damage 9e+01)
      (Variables|/Script/Engine.CharacterMovementComponent|SetMaxWalkSpeed (Variables|Character|GetCharacterMovement) 1e+03)
      (Development|PrintString "awesome powers activate")
      (Utilities|FlowControl|Delay 15.0)
      (Variables|Default|SetBase%20Damage 6e+01)
      (Variables|/Script/Engine.CharacterMovementComponent|SetMaxWalkSpeed (Variables|Character|GetCharacterMovement) 6e+02)
      (Development|PrintString "awesome powers deactivate")
      (Utilities|FlowControl|Delay (Variables|Default|GetAbilityCD1))
      (Variables|Default|Seta1cd true)
      (Development|PrintString "awesome powers ready")
      (else
        (Development|PrintString "cooldown")))))

(event Input|ActionEvents|InputActionAbility2
  (params (Key :type Key%20Structure :default "None"))
  (:Pressed
    (if (Variables|Default|Getfree)
      (if (Variables|Default|Geta2cd)
        (Variables|Default|Setshield true)
        (Variables|Default|Setfree false)
        (Development|PrintString "SHIELD ACTIVE")
        (else
          (Development|PrintString "COOLDOWN")))
      (else
        (Variables|Default|Setrelease%20free false))))
  (:Released
    (if (Variables|Default|Getrelease%20free)
      (if (Variables|Default|Geta2cd)
        (for _array_element (Collision|GetOverlappingActors (Variables|Default|GetSphere) 0 :!class /Script/Engine.PrimitiveComponent)
          (if (not (Actor|ActorHasTag _array_element (Utilities|Array|Get(acopy) (Variables|Default|GetTags))))
            (Utilities|Array|Add (Variables|Default|Gettargets) _array_element)))
        (Variables|Default|Setfinal%20burst (+ (/ (Variables|Default|Getcharge) (Utilities|Array|Length (Variables|Default|Gettargets))) (Variables|Default|Getinit%20burst)))
        (Development|PrintString "BURST")
        (for _array_element_2 (Variables|Default|Gettargets)
          (Game|Damage|ApplyDamage _array_element_2 (Variables|Default|Getfinal%20burst) 0 0)
          (Development|PrintString (Utilities|String|Append (Utilities|GetDisplayName _array_element_2) " DAMAGE:   " (Utilities|String|ToString(Float) (Variables|Default|Getfinal%20burst))) true true "(R=1.000000,G=0.110368,B=0.000000,A=1.000000)"))
        (Variables|Default|Setshield false)
        (Variables|Default|Seta2cd false)
        (Variables|Default|Setcharge 0.0)
        (Variables|Default|Setfinal%20burst 0.0)
        (Utilities|Array|Clear (Variables|Default|Gettargets))
        (Variables|Default|Setfree true)
        (Utilities|FlowControl|Delay 1.0)
        (Variables|Default|Seta2cd true))
      (else
        (Variables|Default|Setrelease%20free true)))))

(fn ConstructionScript
  (|CallParentFunction))