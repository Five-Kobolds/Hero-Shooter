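; BP_TestDummy_Jonah is a test dummy that displays damage taken and can fire a shotgun-style hitscan attack.
; AnyDamage lowers Health, accumulates a total and spawns one BP_DamageNumbers at an Arrow through a DoOnce.
; Once damaged, Tick turns that Arrow relative to the attacker and, after a delay, stops number updates and resets total and DoOnce.
; Fire! waits, then line-traces randomly spread pellets, applying clamped damage with distance falloff and tag-based headshot multipliers.
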(event Custom|ResetDMGNum
  (Utilities|FlowControl|DoOnce false) ; enters at Reset
)

(event Custom|Fire!
  (bind _spread (Variables|Default|GetSpread))
  (bind _spread_2 (Variables|Default|GetSpread))
  (bind _spread_3 (Variables|Default|GetSpread))
  (bind _projectile_spawner (Variables|Default|GetProjectile%20Spawner))
  (bind _returnvalue (Transformation|GetWorldLocation _projectile_spawner))
  (Utilities|FlowControl|Delay 2.0)
  ;[1 1 1] For Each Pellet
  (for _index (range 0 5)
    (bind _outhit (Collision|LineTraceByChannel _returnvalue (+ _returnvalue (* (Math|Vector|GetForwardVector (Transformation|GetWorldRotation _projectile_spawner)) 1.5e+03) (Math|Vector|MakeVector (Math|Random|RandomFloatinRange (* _spread -1.0) _spread) (Math|Random|RandomFloatinRange (* _spread_3 -1.0) _spread_3) (Math|Random|RandomFloatinRange (* _spread_2 -1.0) _spread_2))) "TraceTypeQuery1" false 0 "None"))
    (CallFunction|DamageFalloff (.distance _outhit))
    (Utilities|IsValid (.hitactor _outhit)
      (:Is%20Valid
        (CallFunction|HeadshotDetection (.hitcomponent _outhit))
        (Game|Damage|ApplyDamage (.hitactor _outhit) (Math|Float|Clamp(Float) (* (Variables|Default|GetDamage) (Variables|Default|GetFalloff) (Variables|Default|GetHeadshot%20Multiplier)) 0.0 15.0) 0 self "/Engine/EngineDamageTypes/DmgTypeBP_Environmental.DmgTypeBP_Environmental_C")))))

(event Game|Damage|EventAnyDamage
  (params (Damage :type Float%20%28single-precision%29) (DamageType :type Damage%20Type%20Object%20Reference) (InstigatedBy :type Controller%20Object%20Reference) (DamageCauser :type Actor%20Object%20Reference))
  (Utilities|FlowControl|Sequence
    (:then_0
      (Variables|Default|SetLast_Damage Damage)
      (bind _output_get (Variables|Default|SetHealth (- (Variables|Default|GetHealth) Damage)))
      (Development|PrintString (Utilities|String|ToString(Float) _output_get) false)
      (Variables|Default|SetDMGTotal (+ (Variables|Default|GetDMGTotal) (Variables|Default|GetLast_Damage)))
      (Variables|Default|SetDamageTaken true))
    (:then_1
      (Variables|Default|SetDamage_Cause DamageCauser)
      (Utilities|FlowControl|DoOnce false
        (:Completed
          (bind _returnvalue (Game|SpawnActorfromClass "/Game/Characters/BP_DamageNumbers.BP_DamageNumbers_C" (Transformation|GetWorldTransform (Variables|Default|GetArrow)) "Undefined" self 0))
          (Variables|Default|SetDMG_Number _returnvalue))))))

(event EventTick
  (params (DeltaSeconds :type Float%20%28single-precision%29))
  (bind _dmg_number (Variables|Default|GetDMG_Number))
  (if (Variables|Default|GetDamageTaken)
    (Transformation|SetRelativeRotation (Variables|Default|GetArrow) (Math|Rotator|MakeRotator 0.0 0.0 (- (.yaw (Math|Rotator|FindLookatRotation (Transformation|GetActorLocation) (Transformation|GetActorLocation (Variables|Default|GetDamage_Cause)))) 1.8e+02)) false false)
    (Utilities|FlowControl|Delay 1.0)
    (Utilities|FlowControl|Sequence
      (:then_0
        (if (Utilities|IsValid _dmg_number)
          (bind _asbp_damage_numbers (Utilities|Casting|CastToBP_DamageNumbers _dmg_number))
          (Variables|/Game/Characters/BP_DamageNumbers.BP_DamageNumbers_C|SetUpdating _asbp_damage_numbers false)))
      (:then_1
        (Variables|Default|SetDMGTotal 0.0)
        (CallFunction|ResetDMGNum)))))

(fn ConstructionScript)

(fn DamageFalloff
  (params (HitDistance :type Float%20%28double-precision%29))
  (if (not (> HitDistance 1.5e+02))
    (Variables|Default|SetFalloff 1.0)
    (else
      (Variables|Default|SetFalloff (- 1.0 (/ HitDistance 1e+03))))))

(fn HeadshotDetection
  (params (Hit%20Component :type Actor%20Component%20Object%20Reference))
  (bind _componenttags (Variables|/Script/Engine.ActorComponent|GetComponentTags Hit%20Component))
  (if (not (== (Utilities|Array|Length _componenttags) 0))
    (Variables|Default|SetHeadshot%20Multiplier (Math|Float|SelectFloat 2.0 1.0 (== (Utilities|Array|Get(acopy) _componenttags) "Head")))))