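; BP_TestDummy is a damage test target that shows its Hp on a TextRender, set at construction and updated on each hit.
; AnyDamage subtracts the damage from Hp and prints both values, with no death handling.
; Quinn events toggle custom depth on the UnrealEngineScaleReference component for highlighting, and QuinnCloud removes the "EF" tag after a short delay.
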(event Game|Damage|EventAnyDamage
  (params (Damage :type Float%20%28single-precision%29) (DamageType :type Damage%20Type%20Object%20Reference) (InstigatedBy :type Controller%20Object%20Reference) (DamageCauser :type Actor%20Object%20Reference))
  (Development|PrintString (Utilities|String|Append "" " DAMAGE:   " (Utilities|String|ToString(Float) Damage)) true true "(R=0.746140,G=0.009595,B=1.000000,A=1.000000)")
  (Variables|Default|Sethp (- (Variables|Default|Gethp) Damage))
  (Development|PrintString (Utilities|String|ToString(Float) (Variables|Default|Gethp)))
  (Rendering|Components|TextRender|SetText (Variables|Default|GetTextRender) (Utilities|Text|ToText(Float) (Variables|Default|Gethp) "HalfToEven")))

(event EventQuinnCloud
  (Utilities|FlowControl|Delay 0.5)
  (Utilities|Array|RemoveItem (Variables|Actor|GetTags) "EF"))

(event EventQuinnHighlight
  (Rendering|SetRenderCustomDepth (Variables|Default|GetUnreal_Engine_Scale_Reference self) true))

(event EventQuinnDehighlight
  (Rendering|SetRenderCustomDepth (Variables|Default|GetUnreal_Engine_Scale_Reference self) false))

(fn ConstructionScript
  (Rendering|Components|TextRender|SetText (Variables|Default|GetTextRender) (Utilities|Text|ToText(Float) (Variables|Default|Gethp) "HalfToEven")))