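; Base game mode for a two-team capture point match, moving through pre-game, active and post-game phases.
; Tick runs the phase timer, opens BP_Capture_Point during active play and checks for completion.
; Gated capture updates raise team scores; near the limit, overtime can close the gate and pause timer and win checks until OpenGate is called.
; Completion briefly sets the winning team's message.
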(event Custom|Gamemode_Timer
  (bind _returnvalue (Utilities|Time|GetWorldDeltaSeconds))
  (if (not (Variables|Default|GetInOvertime))
    (Utilities|FlowControl|Delay _returnvalue)
    (bind _output_get (Variables|Default|SetGame_Timer (- (Variables|Default|GetGame_Timer) _returnvalue)))
    (|DebugTimerPrint _output_get
      (:Output
        (if (<= _output_get 0.0)
          (CallFunction|GamemodeProgression))))))

(event Custom|Gamemode%20Progression
  (Variables|Default|SetEnum_GameState (|IncrementEnum))
  (Utilities|FlowControl|DoOnce false) ; enters at Reset
)

(event Custom|Gamemode%20Complete
  (Utilities|FlowControl|DoOnce false
    (:Completed
      (CallFunction|CloseGate)
      (if (> (Variables|Default|GetTeam1_Capture) (Variables|Default|GetTeam2_Capture))
        (Variables|Default|SetWinning%20Team "Team 1 Wins!")
        (else
          (Variables|Default|SetWinning%20Team "Team 2 Wins!")))
      (Utilities|FlowControl|Delay 5.0)
      (Variables|Default|SetWinning%20Team " "))))

(event Custom|CheckIfWin
  (bind _inovertime (Variables|Default|GetInOvertime))
  (bind _returnvalue (not _inovertime))
  (if (and (or (> (Variables|Default|GetTeam1_Capture) 1e+02) (< 1e+02 (Variables|Default|GetTeam2_Capture))) _returnvalue)
    (CallFunction|GamemodeProgression)
    (Variables|Default|SetGameComplete true)
    (elif (and (== (Math|Conversions|ToInteger(Byte) (Variables|Default|GetEnum_GameState)) 3) _returnvalue)
      (Variables|Default|SetGameComplete true))))

(event Custom|AssaultPoint_CaptureUpdate
  (params (Team_Tag :type Name))
  (Utilities|FlowControl|Gate false
    (:Exit
      (Utilities|FlowControl|Delay 0.3)
      (if (not (== Team_Tag "Null"))
        (if (== Team_Tag "Team 1")
          (bind _output_get (Variables|Default|SetTeam1_Capture (+ (Variables|Default|GetTeam1_Capture) 0.25)))
          (else
            (bind _output_get_2 (Variables|Default|SetTeam2_Capture (+ 0.25 (Variables|Default|GetTeam2_Capture))))))
        (if (or (>= _output_get_2 97.5) (>= _output_get 97.5))
          (if (and (>= _output_get 97.5) (>= _output_get_2 97.5))
            (Variables|Default|SetEnum_OvertimeState "NewEnumerator4")
            (elif (== (select (>= _output_get 97.5) 1 0) 1)
              (Variables|Default|SetEnum_OvertimeState "NewEnumerator1")
              (else
                (Variables|Default|SetEnum_OvertimeState "NewEnumerator2"))))
          (bind _returnvalue (Actor|GetActorOfClass "/Game/Defaults/BP_Capture_Point.BP_Capture_Point_C"))
          (Default|TeamPresence _returnvalue)
          (Utilities|FlowControl|DoOnce false
            (:Completed
              (CallFunction|OvertimeFlow (Variables|/Game/Defaults/BP_Capture_Point.BP_Capture_Point_C|GetPointControl (Variables|Default|GetCapture%20Point))))))))))

(event Custom|OvertimeFlow
  (params (ObjectiveControl :type Name))
  (bind _overtimevalid (Variables|Default|GetOvertimeValid))
  (bind _enum_overtimestate (Variables|Default|GetEnum_OvertimeState))
  (bind _returnvalue (Math|Conversions|ToInteger(Byte) _enum_overtimestate))
  (bind _returnvalue_2 (Utilities|Select :Index _returnvalue :Option%200 "None" :Option%201 "Team 1" :Option%202 "Team 2" :Option%203 "Both"))
  (if (or (and _overtimevalid (== ObjectiveControl _returnvalue_2)) (and _overtimevalid (== _returnvalue_2 "Both")))
    (Utilities|FlowControl|Delay 2.7)
    (Variables|Default|SetInOvertime true)
    (CallFunction|CloseGate)))

(event Custom|Close%20Gate
  (Utilities|FlowControl|Gate false) ; enters at Close
)

(event Custom|Open%20Gate
  (Variables|Default|SetInOvertime false)
  (Utilities|FlowControl|Gate false) ; enters at Open
)

(event Custom|Overtime%20Flow%20Reset
  (Utilities|FlowControl|DoOnce false) ; enters at Reset
)

(event EventBeginPlay
  (bind _returnvalue (Actor|GetActorOfClass "/Game/Defaults/BP_Capture_Point.BP_Capture_Point_C"))
  (Variables|Default|SetCapture%20Point _returnvalue)
  (Utilities|FlowControl|Delay 4.0)
  (Variables|Default|SetDefaultPawnClass "/Game/Characters/Support/Suppoer_Ana/B-B.B-B_C")
  (bind _returnvalue_2 (Class|GameplayStatics|CreatePlayer -1))
  (Class|InterfaceAssignTeams|AssignTeam(Message) (Components|GetOwner _returnvalue_2) false))

(event EventTick
  (params (DeltaSeconds :type Float%20%28single-precision%29))
  (bind _enum_gamestate (Variables|Default|GetEnum_GameState))
  (Utilities|FlowControl|Sequence
    (:then_0
      (Utilities|FlowControl|DoOnce false
        (:Completed
          (Variables|Default|SetGame_Timer (Utilities|Select :Index _enum_gamestate :NewEnumerator0 (Variables|Default|GetPreGame_Time) :NewEnumerator1 (Variables|Default|GetActiveGame_Time) :NewEnumerator2 0.0))
          (Development|PrintString "Set Time" true true "(R=1.000000,G=0.472817,B=0.000000,A=1.000000)"))))
    (:then_1
      (switch Utilities|FlowControl|Switch|SwitchonE_GameState _enum_gamestate
        (:NewEnumerator0
          (CallFunction|GamemodeTimer))
        (:NewEnumerator1
          (CallFunction|GamemodeTimer)
          (bind _returnvalue (Actor|GetActorOfClass "/Game/Defaults/BP_Capture_Point.BP_Capture_Point_C"))
          (Variables|/Game/Defaults/BP_Capture_Point.BP_Capture_Point_C|SetObjectiveOpen _returnvalue true))))
    (:then_2
      (if (Variables|Default|GetGameComplete)
        (CallFunction|GamemodeComplete)
        (else
          (CallFunction|CheckifWin))))))

(fn ConstructionScript)