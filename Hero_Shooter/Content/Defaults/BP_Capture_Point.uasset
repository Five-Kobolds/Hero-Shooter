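; Capture point actor for an assault objective, where a team standing in its Box takes control after an uncontested timed capture.
; Overlap events track occupants, recompute team presence from actor tags, and mark overtime valid on the game mode when both teams are present.
; While open and outside overtime, Tick checks the indexed occupant, reporting to the game mode if its team holds the point, otherwise accumulating capture progress.
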(event OnComponentBeginOverlap(Box)
  (params (OverlappedComponent :type Primitive%20Component%20Object%20Reference) (OtherActor :type Actor%20Object%20Reference) (OtherComp :type Primitive%20Component%20Object%20Reference) (OtherBodyIndex :type Integer) (bFromSweep :type Boolean) (SweepResult :type Hit%20Result%20Structure%20%28by%20ref%29))
  (bind _returnvalue (Utilities|Array|Add (Variables|Default|GetActorsPresent) OtherActor))
  (Variables|Default|SetPlayerIndex _returnvalue)
  (CallFunction|TeamPresence false false))

(event OnComponentEndOverlap(Box)
  (params (OverlappedComponent :type Primitive%20Component%20Object%20Reference) (OtherActor :type Actor%20Object%20Reference) (OtherComp :type Primitive%20Component%20Object%20Reference) (OtherBodyIndex :type Integer))
  (Utilities|Array|RemoveItem (Variables|Default|GetActorsPresent) OtherActor)
  (CallFunction|TeamPresence false false))

(event Custom|TeamPresence
  (params (Team%201 :type Boolean) (Team%202 :type Boolean))
  (for _array_element (Variables|Default|GetActorsPresent)
    (bind _output_get (Variables|Default|SetTeam%201 (or (Utilities|Array|ContainsItem (Variables|/Script/Engine.Actor|GetTags _array_element) "Team 1") Team%201)))
    (bind _output_get_2 (Variables|Default|SetTeam%202 (or (Utilities|Array|ContainsItem (Variables|/Script/Engine.Actor|GetTags _array_element) "Team 2") Team%202)))
    (bind _asbp_game_mode_base (Utilities|Casting|CastToBP_GameMode_Base (Game|GetGameMode)))
    (Variables|/Game/Defaults/BP_GameMode_Base.BP_GameMode_Base_C|SetOvertimeValid _asbp_game_mode_base (and _output_get_2 _output_get))))

(event Custom|TeamCapture
  (bind _output_get (Variables|Default|SetCaptureProgress (Math|Float|Clamp(Float) (+ (Utilities|Time|GetWorldDeltaSeconds) (Variables|Default|GetCaptureProgress)) 0.0 8.0)))
  (if (== _output_get 8.0)
    (Variables|Default|SetPointControl (Utilities|Array|Get(acopy) (Variables|/Script/Engine.Actor|GetTags (Utilities|Array|Get(acopy) (Variables|Default|GetActorsPresent) (Variables|Default|GetPlayerIndex)))))
    (Variables|Default|SetCaptureProgress 0.0)))

(event Custom|GameplayOvertime
  (Variables|Default|SetOvertime true))

(event EventTick
  (params (DeltaSeconds :type Float%20%28single-precision%29))
  (if (Math|Boolean|ANDBoolean (Variables|Default|GetObjectiveOpen) (>= (Utilities|Array|Length (Variables|Default|GetActorsPresent)) 1) (not (Variables|Default|GetOvertime)))
    (if (Utilities|Array|ContainsItem (Variables|/Script/Engine.Actor|GetTags (Utilities|Array|Get(acopy) (Variables|Default|GetActorsPresent) (Variables|Default|GetPlayerIndex))) (Variables|Default|GetPointControl))
      (bind _asbp_game_mode_base (Utilities|Casting|CastToBP_GameMode_Base (Game|GetGameMode)))
      (Default|AssaultPointCaptureUpdate _asbp_game_mode_base (Variables|Default|GetPointControl))
      (elif (Class|KismetMathLibrary|XORBoolean (Variables|Default|GetTeam%201) (Variables|Default|GetTeam%202))
        (CallFunction|TeamCapture)))))

(fn ConstructionScript)